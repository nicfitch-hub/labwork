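; NewSceneComponent is a component Blueprint that cycles two counters, Brightnessness and Darknessness, with no visible use of their values in the graph.
; Each Tick raises Brightnessness by one until it reaches 1000, then raises Darknessness the same way, then resets both to zero.
; The count advances per frame without Delta Seconds, so the cycle length depends on frame rate.
; BeginPlay is an unused, disabled stub.
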(event EventBeginPlay)

(event EventTick
  (params (DeltaSeconds :type Float%20%28single-precision%29))
  (if (== (Variables|Default|GetBrightnessness) 1000)
    (if (== (Variables|Default|GetDarknessness) 1000)
      (Variables|Default|SetBrightnessness 0)
      (Variables|Default|SetDarknessness 0)
      (else
        (Math|Integer|IncrementInt (Variables|Default|GetDarknessness))))
    (else
      (Math|Integer|IncrementInt (Variables|Default|GetBrightnessness)))))