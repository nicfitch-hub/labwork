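; THESUN is a sun actor that sets its point light's intensity every tick, apparently meant as a repeating brighten and dim cycle.
; Two per-tick counters, Brightnessness then Darknessness, each count to 1000 before both reset.
; Intensity reads from increment and decrement nodes on CurentBright that never execute, so the ramp is not actually driven.
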(event EventTick
  (params (DeltaSeconds :type Float%20%28single-precision%29))
  (if (== (Variables|Default|GetBrightnessness) 1000)
    (if (== (Variables|Default|GetDarknessness) 1000)
      (Variables|Default|SetBrightnessness 0)
      (Variables|Default|SetDarknessness 0)
      (else
        (Math|Integer|IncrementInt (Variables|Default|GetDarknessness)
          (:%20%20
            (Rendering|Components|Light|SetIntensity (Variables|Default|GetPointLight) (Math|Conversions|ToFloat(Integer) (stale _result)))))))
    (else
      (Math|Integer|IncrementInt (Variables|Default|GetBrightnessness)
        (:%20%20
          (Rendering|Components|Light|SetIntensity (Variables|Default|GetPointLight) (Math|Conversions|ToFloat(Integer) (stale _result))))))))

(event EventBeginPlay)

(event Collision|EventActorBeginOverlap
  (params (OtherActor :type Actor%20Object%20Reference)))

(fn ConstructionScript)