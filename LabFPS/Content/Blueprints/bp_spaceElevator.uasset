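; Space elevator actor that the player rides up or down with the U and D keys after collecting exactly three coins.
; Overlap with the first-person character enables its key input and stores that character for the coin check; leaving disables input.
; Each key plays its own timeline, lerping the cube from its current location toward a fixed high or low world Z, so easing compounds every update.
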(event Collision|EventActorBeginOverlap
  (params (OtherActor :type Actor%20Object%20Reference))
  (bind _asbp_first_person_character (Utilities|Casting|CastToBP_FirstPersonCharacter OtherActor))
  (Input|EnableInput (Game|GetPlayerController 0)))

(event EventTick
  (params (DeltaSeconds :type Float%20%28single-precision%29)))

(event Collision|EventActorEndOverlap
  (params (OtherActor :type Actor%20Object%20Reference))
  (Utilities|Casting|CastToBP_FirstPersonCharacter OtherActor)
  (Input|DisableInput (Game|GetPlayerController 0)))

(event Input|KeyboardEvents|U
  (params (Key :type Key%20Structure :default "None"))
  (bind _cube (Variables|Default|GetCube))
  (bind _returnvalue (Transformation|GetWorldLocation _cube))
  (:Pressed
    (if (== (Variables|/Game/FirstPerson/Blueprints/BP_FirstPersonCharacter.BP_FirstPersonCharacter_C|GetPlayerCoins (stale Collision|EventActorBeginOverlap _asbp_first_person_character)) 3)
      (bind _movement (Timeline|Timeline Play)
        (:Update
          (Transformation|SetWorldLocation (Variables|Default|GetCube) (Math|Vector|Lerp(Vector) (Math|Vector|MakeVector (.x _returnvalue) (.y _returnvalue) (.z _returnvalue)) (Math|Vector|MakeVector (.x _returnvalue) (.y _returnvalue) 1e+03) _movement) false false))))))

(event Input|KeyboardEvents|D
  (params (Key :type Key%20Structure :default "None"))
  (bind _cube (Variables|Default|GetCube))
  (bind _returnvalue (Transformation|GetWorldLocation _cube))
  (:Pressed
    (if (== (Variables|/Game/FirstPerson/Blueprints/BP_FirstPersonCharacter.BP_FirstPersonCharacter_C|GetPlayerCoins (stale Collision|EventActorBeginOverlap _asbp_first_person_character)) 3)
      (bind _movement (Timeline|Timeline_0 Play)
        (:Update
          (Transformation|SetWorldLocation (Variables|Default|GetCube) (Math|Vector|Lerp(Vector) (Math|Vector|MakeVector (.x _returnvalue) (.y _returnvalue) (.z _returnvalue)) (Math|Vector|MakeVector (.x _returnvalue) (.y _returnvalue) -1e+03) _movement) false false))))))

(fn ConstructionScript)