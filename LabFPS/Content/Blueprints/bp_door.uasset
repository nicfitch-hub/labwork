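; Door actor Blueprint that opens by sliding its Cube along the world X axis when an actor overlaps its linked button.
; On BeginPlay it finds the nearest Bp_button by distance and binds Open to that button's begin-overlap event.
; Open plays a timeline that lerps the Cube from its current location toward a fixed world X, re-sampling the start each update.
; No closing logic is present.
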(event Custom|Open
  (params (OverlappedActor :type Actor%20Object%20Reference) (OtherActor :type Actor%20Object%20Reference))
  (bind _cube (Variables|Default|GetCube))
  (bind _returnvalue (Transformation|GetWorldLocation _cube))
  (Development|PrintString "Door Open")
  (bind _movement (Timeline|Timeline Play)
    (:Update
      (Transformation|SetWorldLocation (Variables|Default|GetCube) (Math|Vector|Lerp(Vector) (Math|Vector|MakeVector (.x _returnvalue) (.y _returnvalue) (.z _returnvalue)) (Math|Vector|MakeVector -1e+04 (.y _returnvalue) (.z _returnvalue)) _movement) false false))))

(event Collision|EventActorBeginOverlap
  (params (OtherActor :type Actor%20Object%20Reference)))

(event EventTick
  (params (DeltaSeconds :type Float%20%28single-precision%29)))

(event EventBeginPlay
  (Variables|Default|SetClosest 1e+06)
  (Variables|Default|SetArraybest 0)
  (bind _outactors (Actor|GetAllActorsOfClass "/Game/Blueprints/bp_button.bp_button_C"))
  (for (_array_element _array_index) _outactors
    (if (> (Variables|Default|GetClosest) (Transformation|GetDistanceTo _array_element))
      (Variables|Default|SetClosest (Transformation|GetDistanceTo _array_element))
      (Variables|Default|SetArraybest _array_index)))
  (Collision|BindEventtoOnActorBeginOverlap (Utilities|Array|Get(acopy) _outactors (Variables|Default|GetArraybest)) (delegate Custom|Open)))

(fn ConstructionScript)