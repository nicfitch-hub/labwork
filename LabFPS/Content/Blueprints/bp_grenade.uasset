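; Grenade Blueprint that, after a short fixed fuse, blasts nearby physics objects outward.
; On BeginPlay it nudges its Sphere component with the first-person character's unscaled forward vector as an impulse, then waits.
; It then gathers PhysicsBody components by sphere overlap and gives each a constant-falloff radial impulse from the Sphere's location, using a smaller radius than the search.
; The graph applies no damage or effects and never destroys the grenade.
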(event EventBeginPlay
  (bind _sphere (Variables|Default|GetSphere))
  (bind _returnvalue (Transformation|GetWorldLocation _sphere))
  (bind _returnvalue_2 (Actor|GetActorOfClass "/Game/FirstPerson/Blueprints/BP_FirstPersonCharacter.BP_FirstPersonCharacter_C"))
  (Physics|AddImpulse (Variables|Default|GetSphere) (Transformation|GetActorForwardVector _returnvalue_2) "None" false)
  (Utilities|FlowControl|Delay 3.0)
  (bind _outcomponents (Collision|SphereOverlapComponents _returnvalue 5e+03 (Utilities|Array|MakeArray "ObjectTypeQuery4")))
  (for _array_element _outcomponents
    (Physics|AddRadialImpulse _array_element _returnvalue 3.5e+03 5e+05 "RIF_Constant" false)))

(event Collision|EventActorBeginOverlap
  (params (OtherActor :type Actor%20Object%20Reference)))

(event EventTick
  (params (DeltaSeconds :type Float%20%28single-precision%29)))

(fn ConstructionScript)