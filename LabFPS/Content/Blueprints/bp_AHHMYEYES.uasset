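; Light actor that sets its point light to high intensity when the nearest Bp_button is overlapped.
; On BeginPlay it searches all Bp_button actors by distance using Closest and Arraybest, then binds Open to the selected button's begin-overlap event.
; Unconnected leftovers include the search variable initialisation and a Bp_button2 binding to a second, far brighter intensity event.
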(event Custom|Open
  (params (OverlappedActor :type Actor%20Object%20Reference) (OtherActor :type Actor%20Object%20Reference))
  (Rendering|Components|Light|SetIntensity (Variables|Default|GetPointLight) 5e+04))

(event Custom|CustomEvent_1
  (params (OverlappedActor :type Actor%20Object%20Reference) (OtherActor :type Actor%20Object%20Reference))
  (Rendering|Components|Light|SetIntensity (Variables|Default|GetPointLight) 9e+06))

(event Collision|EventActorBeginOverlap
  (params (OtherActor :type Actor%20Object%20Reference)))

(event EventTick
  (params (DeltaSeconds :type Float%20%28single-precision%29)))

(event EventBeginPlay
  (bind _outactors (Actor|GetAllActorsOfClass "/Game/Blueprints/bp_button.bp_button_C"))
  (for (_array_element _array_index) _outactors
    (if (> (Variables|Default|GetClosest) (Transformation|GetDistanceTo _array_element))
      (Variables|Default|SetClosest (Transformation|GetDistanceTo _array_element))
      (Variables|Default|Setarraybest _array_index)))
  (Collision|BindEventtoOnActorBeginOverlap (Utilities|Array|Get(acopy) _outactors (Variables|Default|GetArraybest)) (delegate Custom|Open)))

(fn ConstructionScript)