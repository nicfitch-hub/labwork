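; Grenade spawner actor that drops a Bp_grenade at its own transform when its nearest button is overlapped.
; On BeginPlay it searches all Bp_button actors for the closest one and binds Open to that button's OnActorBeginOverlap.
; Each overlap spawns another grenade, with no check on the overlapping actor, so pairing depends purely on level placement.
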(event Custom|Open
  (params (OverlappedActor :type Actor%20Object%20Reference) (OtherActor :type Actor%20Object%20Reference))
  (Game|SpawnActorfromClass "/Game/Blueprints/bp_grenade.bp_grenade_C" (Transformation|GetActorTransform) "Undefined" "MultiplyWithRoot" 0 0))

(event EventBeginPlay
  (Variables|Default|SetClosest 1e+06)
  (Variables|Default|Setarraybest 0)
  (bind _outactors (Actor|GetAllActorsOfClass "/Game/Blueprints/bp_button.bp_button_C"))
  (for (_array_element _array_index) _outactors
    (if (> (Variables|Default|GetClosest) (Transformation|GetDistanceTo _array_element))
      (Variables|Default|SetClosest (Transformation|GetDistanceTo _array_element))
      (Variables|Default|Setarraybest _array_index)))
  (Collision|BindEventtoOnActorBeginOverlap (Utilities|Array|Get(acopy) _outactors (Variables|Default|GetArraybest)) (delegate Custom|Open)))

(event Collision|EventActorBeginOverlap
  (params (OtherActor :type Actor%20Object%20Reference)))

(event EventTick
  (params (DeltaSeconds :type Float%20%28single-precision%29)))

(fn ConstructionScript)