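; An actor Blueprint, apparently an unfinished save point, with custom events for loading and saving a bp_gameSave object.
; The load event checks slot "demosave" but loads "obSave", casts the result without using it, and prints "no" when the check fails.
; The save event is empty.
; Nodes that would save the Groovy value to "obSave" and set the actor transform are disconnected, so nothing is saved or restored.
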(event Custom|load%20gane
  (bind _returnvalue (SaveGame|DoesSaveGameExist "demosave"))
  (if _returnvalue
    (bind _returnvalue_2 (SaveGame|LoadGamefromSlot "obSave"))
    (Utilities|Casting|CastTobp_gameSave _returnvalue_2)
    (else
      (Development|PrintString "no"))))

(event Custom|Save%20Gmae)

(event EventBeginPlay)

(event Collision|EventActorBeginOverlap
  (params (OtherActor :type Actor%20Object%20Reference)))

(event EventTick
  (params (DeltaSeconds :type Float%20%28single-precision%29)))

(fn ConstructionScript)